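; Classic race game mode, apparently a work in progress, meant to manage local players, lap and checkpoint totals, and a race stopwatch.
; BeginPlay creates a local player and caches player controllers of that class, then loops over them doing nothing.
; The Timer event would add delta time per controller and race component once started, printing it.
; Race component and HUD setup, delayed start and Timer's call sit in unconnected chains that never run.
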(event Custom|Timer
  (if (Variables|Default|GethasRaceStarted?)
    (for _array_element (Variables|Default|GetLocal%20Players%20Player%20Controller)
      (Utilities|IsValid _array_element
        (:Is%20Valid
          (for _array_element_2 (Variables|Default|GetLocal%20Players%20Race%20Component)
            (Utilities|IsValid _array_element_2
              (:Is%20Valid
                (bind _output_get (Variables|Default|SetCronometer (+ (Variables|Default|GetCronometer) (Utilities|Time|GetWorldDeltaSeconds))))
                (Development|PrintString (Utilities|String|ToString(Float) _output_get))))))))))

(event EventBeginPlay
  (bind _returnvalue (Class|GameplayStatics|CreatePlayer -1))
  (Utilities|IsValid _returnvalue
    (:Is%20Valid
      (bind _outactors (Actor|GetAllActorsOfClass (Utilities|GetClass _returnvalue)))
      (bind _output_get (Variables|Default|SetLocal%20Players%20Player%20Controller _outactors))
      (for _array_element _output_get
        _))))

(event EventTick
  (params (DeltaSeconds :type Float%20%28single-precision%29)))

(fn ConstructionScript)